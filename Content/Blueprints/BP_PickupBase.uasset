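; Base pickup actor that hands its Item to whoever interacts with it, then removes itself from the world.
; Sphere1 begin and end overlaps toggle the overlapping actor's BP_InteractionComponent through OnInteractableOverlap, with validity and player-character checks left unconnected.
; Interact calls PickupMessage on the interactor with the Item, destroys the pickup and returns true.
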(event OnComponentBeginOverlap(Sphere1)
  (params (OverlappedComponent :type Primitive%20Component%20Object%20Reference) (OtherActor :type Actor%20Object%20Reference) (OtherComp :type Primitive%20Component%20Object%20Reference) (OtherBodyIndex :type Integer) (bFromSweep :type Boolean) (SweepResult :type Hit%20Result%20Structure%20%28by%20ref%29))
  (if true
    (Default|OnInteractableOverlap (Actor|GetComponentbyClass OtherActor "/Game/Blueprints/BP_InteractionComponent.BP_InteractionComponent_C") true)))

(event OnComponentEndOverlap(Sphere1)
  (params (OverlappedComponent :type Primitive%20Component%20Object%20Reference) (OtherActor :type Actor%20Object%20Reference) (OtherComp :type Primitive%20Component%20Object%20Reference) (OtherBodyIndex :type Integer))
  (if true
    (Default|OnInteractableOverlap (Actor|GetComponentbyClass OtherActor "/Game/Blueprints/BP_InteractionComponent.BP_InteractionComponent_C") false)))

(event EventBeginPlay)

(event EventTick
  (params (DeltaSeconds :type Float%20%28single-precision%29)))

(fn ConstructionScript)

(fn Interact
  (params (Interactor :type Character%20Object%20Reference))
  ;[0.15 0.15 0.15 0.5] Everything you want to have happen on an interact
  (Class|BPIPickup|Pickup(Message) Interactor (Variables|Default|GetItem))
  (Actor|DestroyActor)
  (return true))