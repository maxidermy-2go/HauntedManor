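; Door actor that receives character interactions and exposes an OpenDoor event to set its open state.
; Interacts only forwards the Character to the parent class implementation.
; OpenDoor stores the Open flag and plays DoorOpenTimeline when true; false only clears the flag, with no reverse playback.
; The graph shows no timeline update logic, so no door movement is driven here.
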(event Custom|Open%20Door
  (params (Open :type Boolean))
  (if Open
    (Variables|Default|SetOpen true)
    (Timeline|Door%20Open%20Timeline Play)
    (else
      (Variables|Default|SetOpen false))))

(event EventBeginPlay
  (|CallParentFunction) ; This node is disabled and will not be called.\nDrag off pins to build functionality.
)

(event Collision|EventActorBeginOverlap
  (params (OtherActor :type Actor%20Object%20Reference)))

(event EventTick
  (params (DeltaSeconds :type Float%20%28single-precision%29))
  (|CallParentFunction DeltaSeconds) ; This node is disabled and will not be called.\nDrag off pins to build functionality.
)

(event EventInteracts
  (params (Character :type Actor%20Object%20Reference))
  (|CallParentFunction Character))

(fn ConstructionScript
  (|CallParentFunction))