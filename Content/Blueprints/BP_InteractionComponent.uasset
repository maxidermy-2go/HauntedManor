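; Interaction component that detects when the player is looking at a nearby actor tagged "Interactable".
; Overlap events keep a count that starts a looping sight-check timer while above zero and clears it otherwise, avoiding Tick.
; Each check sphere-traces a short distance from the deprojected screen center, setting or clearing HitActor and CanInteract, with debug drawing and prints.
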(event Custom|On%20Interactable%20Overlap
  (params (Overlaps :type Boolean))
  ;[0.15 0.15 0.15 0.5] When within object collision
  (Utilities|FlowControl|Sequence
    (:then_0
      (bind _output_get (Variables|Default|SetOverlap%20Count (+ (Variables|Default|GetOverlap%20Count) (select Overlaps 1 -1))))
      (Development|PrintString (Utilities|String|ToString(Integer) _output_get)))
    (:then_1
      (CallFunction|DrawTrace (> (Variables|Default|GetOverlap%20Count) 0)))))

(event Custom|Draw%20Trace
  (params (Draw%20Trace :type Boolean))
  (if Draw%20Trace
    (bind _returnvalue (Utilities|Time|SetTimerbyFunctionName 0 "Detect Sight" 0.1 true))
    (Variables|Default|SetTraceTimer _returnvalue)
    (else
      (Utilities|Time|ClearandInvalidateTimerbyHandle (Variables|Default|GetTraceTimer)))))

(event Custom|Detect%20Sight
  (bind (_worldlocation _returnvalue) (CallFunction|CalculateTraceStartEnd))
  ;[0.15 0.15 0.15 0.5] can look at and interact with object
  (bind (_outhit _returnvalue_2) (Collision|SphereTraceByChannel _worldlocation _returnvalue 5.0 "TraceTypeQuery1" false 0 "ForDuration" true "(R=1.000000,G=0.000000,B=0.000000,A=1.000000)" "(R=0.000000,G=1.000000,B=0.000000,A=1.000000)" 0.1))
  (if _returnvalue_2
    (if (Actor|ActorHasTag (.HitActor (Collision|BreakHitResult _outhit)) "Interactable")
      (Variables|Default|SetHit%20Actor (.HitActor (Collision|BreakHitResult _outhit)))
      (Variables|Default|SetCan%20Interact true)
      (Development|PrintString "Looking")
      (else
        (Variables|Default|SetHit%20Actor 0 :!label _label)
        (Variables|Default|SetCan%20Interact false)
        (Development|PrintString "Not Looking")))
    (else
      (goto _label))))

(event EventBeginPlay)

(event EventTick
  (params (DeltaSeconds :type Float%20%28single-precision%29)))

(fn CalculateTraceStartEnd
  (bind _returnvalue (Game|GetPlayerController 0))
  (bind (_sizex _sizey) (HUD|GetViewportSize _returnvalue))
  (bind _returnvalue_2 (/ _sizey 2))
  (bind _returnvalue_3 (/ _sizex 2))
  (bind _returnvalue_4 (Math|Conversions|ToFloat(Integer) _returnvalue_3))
  (bind _returnvalue_5 (Math|Conversions|ToFloat(Integer) _returnvalue_2))
  (bind (_worldlocation _worlddirection) (Class|PlayerController|DeprojectScreenPositiontoWorld _returnvalue _returnvalue_4 _returnvalue_5))
  (return _worldlocation (+ (* _worlddirection 2.5e+02) _worldlocation)))