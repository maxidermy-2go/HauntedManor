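; BP_EnemyAI is an enemy AI pawn that detects the player through PawnSensing.
; Seeing a BP_FirstPersonCharacter sets the HasSeenPlayer blackboard key to true on its AI controller, and nothing here clears it.
; A FollowPlayer event moves it toward the player with AIMoveTo, but its only call in this graph is unreachable.
; Tick's movement stop never fires because its condition is constant, and noise hearing is empty.
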(event OnHearNoise(PawnSensing)
  (params (Instigator :type Pawn%20Object%20Reference) (Location :type Vector%20%28by%20ref%29 :default "0, 0, 0") (Volume :type Float%20%28single-precision%29)))

(event OnSeePawn(PawnSensing)
  (params (Pawn :type Pawn%20Object%20Reference))
  (Utilities|Casting|CastToBP_FirstPersonCharacter Pawn)
  (AI|Components|Blackboard|SetValueasBool (AI|GetBlackboard (AI|GetAIController self)) (Utilities|Name|MakeLiteralName "HasSeenPlayer") true))

(event Custom|FollowPlayer
  (Variables|Default|SetcanAttack? true)
  (if true
    (AI|AIMoveTo self "0, 0, 0" (Game|GetPlayerCharacter 0) 1.5e+02 false
      (:OnSuccess
        (if (Variables|Default|GetcanAttack?)
          (Variables|Default|SetcanAttack? true))))
    (else
      (Variables|Default|SetisSeeingPlayer? false))))

(event EventBeginPlay)

(event Collision|EventActorBeginOverlap
  (params (OtherActor :type Actor%20Object%20Reference)))

(event EventTick
  (params (DeltaSeconds :type Float%20%28single-precision%29))
  (if (not true)
    (Components|Movement|StopMovementImmediately (Variables|Character|GetCharacterMovement))))

(fn ConstructionScript)