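; BP_Clue is an interactable clue actor that a character can pick up.
; Its Interacts event calls PickUpItem, which finds the character's first StaticMeshComponent by a None tag and checks that its current mesh is valid.
; If so, that component receives the clue's InteractableMesh mesh and PickOrientation relative transform, and the clue actor destroys itself.
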(event Custom|PickUp%20Item
  (params (Character :type Actor%20Object%20Reference))
  (bind _returnvalue (Actor|GetComponentsbyTag Character "/Script/Engine.StaticMeshComponent" "None"))
  (bind _output (Utilities|Array|Get(acopy) _returnvalue))
  ;[0.15 0.15 0.15 0.5] Pickup logic
  (if (Utilities|IsValid (Variables|/Script/Engine.StaticMeshComponent|GetStaticMesh _output))
    (Components|StaticMesh|SetStaticMesh _output (Variables|/Script/Engine.StaticMeshComponent|GetStaticMesh (Variables|Default|GetInteractable%20Mesh)))
    (Transformation|SetRelativeTransform _output (Variables|Default|GetPick%20Orientation) false false)
    (Actor|DestroyActor)))

(event EventBeginPlay
  (|CallParentFunction) ; This node is disabled and will not be called.\nDrag off pins to build functionality.
)

(event Collision|EventActorBeginOverlap
  (params (OtherActor :type Actor%20Object%20Reference)))

(event EventTick
  (params (DeltaSeconds :type Float%20%28single-precision%29))
  (|CallParentFunction DeltaSeconds) ; This node is disabled and will not be called.\nDrag off pins to build functionality.
)

(event EventInteracts
  (params (Character :type Actor%20Object%20Reference))
  (CallFunction|PickUpItem Character))

(fn ConstructionScript
  (|CallParentFunction))