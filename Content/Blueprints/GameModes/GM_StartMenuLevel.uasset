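; Game mode for the start menu level that creates and shows the main menu widget on BeginPlay.
; Its events open the first level by name or swap between the main menu and options menu by toggling widget visibility.
; The options widget is created on first request and cached for reuse, while the main menu is collapsed rather than removed.
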(event Custom|LoadTheFirstLevel
  (Game|OpenLevel(byName) (Variables|Default|GetFirstLevelName))
  (Development|PrintString "Level Transition"))

(event Custom|LoadtheOptionsMenu
  (Utilities|IsValid (Variables|Default|GetWidgetOptionsMenu)
    (:Is%20Valid
      (Widget|SetVisibility (Variables|Default|GetWidgetOptionsMenu) "Visible"))
    (:Is%20Not%20Valid
      (bind _returnvalue (UserInterface|CreateWidget "/Game/Blueprints/WBP/WBP_Options.WBP_Options_C"))
      (bind _output_get (Variables|Default|SetWidgetOptionsMenu _returnvalue))
      (UserInterface|Viewport|AddtoViewport (Variables|Default|GetWidgetOptionsMenu) 0)))
  (Widget|SetVisibility (Variables|Default|GetWidgetMainMenu) "Collapsed"))

(event Custom|SwitchtoStart
  (Widget|SetVisibility (Variables|Default|GetWidgetOptionsMenu) "Collapsed")
  (Widget|SetVisibility (Variables|Default|GetWidgetMainMenu) "Visible"))

(event EventBeginPlay
  (bind _returnvalue (UserInterface|CreateWidget "/Game/Blueprints/WBP/WBP_StartMenu.WBP_StartMenu_C" (Game|GetPlayerController 0)))
  (Variables|Default|SetWidgetMainMenu _returnvalue)
  (UserInterface|Viewport|AddtoViewport _returnvalue 0))

(event EventTick
  (params (DeltaSeconds :type Float%20%28single-precision%29)))

(fn ConstructionScript)